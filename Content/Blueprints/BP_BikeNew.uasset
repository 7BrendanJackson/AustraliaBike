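; Bike actor that moves along the BP_TrackSpline spline, driven by a Bluetooth cycling trainer's wheel RPM.
; BeginPlay starts BLE scanning, binds connection-state debug prints, adds a debug widget and input mapping, and snaps to the spline.
; Each Tick smooths normalised RPM into a per-frame distance step, wraps it, adds move-forward input, then exp-decays location toward that point while snapping rotation.
; A resistance test is left unconnected.
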(event `self.ReceiveBeginPlay`
  (bind _returnvalue (`CyclingPowerBLESubsystem.Get`))
  (bind _spline (`self.Spline`))
  (`CyclingPowerBLESubsystem.StartScanning` _returnvalue)
  (add `CyclingPowerBLESubsystem.OnConnectionStateChanged` _returnvalue (`|CreateDelegate` :!event `ConnectionChange`))
  (bind _returnvalue_2 (`|CreateWidget` "/Game/Blueprints/WBP_DebugBike.WBP_DebugBike_C" null self))
  (`UserWidget.AddToViewport` _returnvalue_2 0)
  (bind _returnvalue_3 (`GameplayStatics.GetActorOfClass` "/Game/Blueprints/BP_TrackSpline.BP_TrackSpline_C"))
  (set `self.Spline` (`/Game/Blueprints/BP_TrackSpline.Spline` _returnvalue_3))
  (`EnhancedInputSubsystemInterface.AddMappingContext` (pcsubsystem `EnhancedInputLocalPlayerSubsystem` (`GameplayStatics.GetPlayerController` 0)) "/Game/Input/IM_Controls.IM_Controls" 0 (struct))
  (`self.K2_SetActorLocationAndRotation` (`SplineComponent.GetLocationAtDistanceAlongSpline` _spline (`self.Distance`) "World") (`SplineComponent.GetRotationAtDistanceAlongSpline` _spline (`self.Distance`) "World")))

(event `ConnectionChange`
  (params (NewState :type "ECyclingPowerConnectionState Enum" :default "Disconnected"))
  (`KismetSystemLibrary.PrintString` (`|GetEnumeratorNameAsString` NewState) true true (select `ECyclingPowerConnectionState` NewState :`Disconnected` (struct :`R` 1.0 :`A` 1.0) :`Scanning` (struct :`R` 1.0 :`G` 0.559178 :`A` 1.0) :`Connecting` (struct :`G` 0.96731 :`B` 1.0 :`A` 1.0) :`Connected` (struct :`G` 1.0 :`B` 0.002 :`A` 1.0) :!type "LinearColor Structure") 5000.0 "Noasdasdasne")
  (if (select `ECyclingPowerConnectionState` NewState :`Connected` true)
    _))

(event `self.ReceiveTick`
  (params (DeltaSeconds :type "Float (single-precision)"))
  (bind _spline (`self.Spline`))
  (`self.CalcValues`)
  (set `self.Distance` (+ (mod (+ (`self.Distance`) (`self.CurrentBikeSpeed`)) (`SplineComponent.GetSplineLength` (`self.Spline`))) (* (`|GetInputActionValue`) 100.0)))
  (`self.K2_SetActorLocationAndRotation` (`/Game/Data/BPFL_Math.ExpDecayVector` (`self.K2_GetActorLocation`) (`SplineComponent.GetLocationAtDistanceAlongSpline` _spline (`self.Distance`) "World") 2.0) (`SplineComponent.GetRotationAtDistanceAlongSpline` _spline (`self.Distance`) "World")))

(fn `CalcValues`
  (bind (_returnvalue_instantaneouspower _returnvalue_bhascadence _returnvalue_cadencerpm _returnvalue_bhasbalance _returnvalue_pedalpowerbalancepercent _returnvalue_bhastorque _returnvalue_accumulatedtorquenm _returnvalue_bhaswheelrpm _returnvalue_wheelrpm) (break `CyclingPowerData` (`CyclingPowerBLESubsystem.GetLastData` (`CyclingPowerBLESubsystem.Get`))))
  (bind _returnvalue (`/Game/Data/BPFL_Math.ExpDecayFloat` (`self.CurrentBikeSpeedNormalised`) (/ _returnvalue_wheelrpm (`self.BikeMaxSpeedOutput`)) 0.2))
  (bind _output_get (set `self.CurrentBikeSpeedNormalised` _returnvalue))
  (set `self.CurrentBikeSpeed` (* _output_get (`self.BikeSpeed`))))

(fn `UserConstructionScript`)