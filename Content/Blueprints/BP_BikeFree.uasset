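; Free-roaming bike actor driven by a physical bike speed sensor and steered with Tobii head tracking.
; Each tick it moves forward without sweep by the raw km/h reading, not scaled by delta time.
; Yaw averages clamped head side offset and roll, applies a deadzone, then scales by delta time, rotation speed and normalised bike speed.
; The head roll captured at BeginPlay is stored but never used in steering.
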(event `self.ReceiveBeginPlay`
  (set `self.HeadCentre` (.roll (`.Rotation` (break `TobiiHeadPoseData` (`TobiiSubsystem.GetHeadPoseData` (subsystem `TobiiSubsystem`)))))))

(event `self.ReceiveTick`
  (params (DeltaSeconds :type "Float (single-precision)"))
  (`self.CalcSpeed`)
  (`self.K2_AddActorWorldOffset` (* (`self.CurrentBikeSpeed`) (`self.GetActorForwardVector`)))
  (`self.K2_AddActorLocalRotation` (`KismetMathLibrary.MakeRotator` 0.0 0.0 (`self.CalcRotation`))))

(event `self.BikeSensor.OnBikeConnected`
  (`KismetSystemLibrary.PrintString` "Bike Connected" true true (struct :`G` 1.0 :`A` 1.0) 5.0))

(fn `CalcRotation`
  (returns (RotationAmount :type "Float (double-precision)"))
  (locals (Value :type "Float (double-precision)"))
  (bind _headtiltmax (`self.HeadTiltMax`))
  (bind _headsidemax (`self.HeadSideMax`))
  (bind _returnvalue (`TobiiSubsystem.GetHeadPoseData` (subsystem `TobiiSubsystem`)))
  (bind _returnvalue_2 (* (`GameplayStatics.GetWorldDeltaSeconds`) (`self.RotationAmount`) (`self.RotationSpeed`) (`self.CurrentBikeSpeedNormalised`)))
  (bind _output_get (set `local.Value` (/ (+ (/ (`KismetMathLibrary.FClamp` (.y (break `TobiiHeadPoseData` _returnvalue)) (* _headsidemax -1.0) _headsidemax) _headsidemax) (/ (`KismetMathLibrary.FClamp` (.roll (`.Rotation` (break `TobiiHeadPoseData` _returnvalue))) (* _headtiltmax -1.0) _headtiltmax) _headtiltmax)) 2.0)))
  (if (<= (`KismetMathLibrary.Abs` _output_get) (`self.Deadzone`))
    (set `self.RotationAmount` 0.0)
    (else
      (set `self.RotationAmount` _output_get)))
  (`KismetSystemLibrary.PrintString` (`KismetStringLibrary.Conv_DoubleToString` _returnvalue_2))
  (return _returnvalue_2))

(fn `CalcSpeed`
  (locals (Value :type "Float (double-precision)"))
  (set `self.CurrentBikeSpeed` (`BikeSensorComponent.GetSpeedKph` (`self.BikeSensor`)))
  (bind _output_get (set `self.CurrentBikeSpeedNormalised` (/ (`self.CurrentBikeSpeed`) (`self.BikeMaxSpeedOutput`))))
  (`KismetSystemLibrary.PrintString` (`KismetStringLibrary.Conv_DoubleToString` _output_get) true true (struct :`G` 0.66 :`B` 1.0 :`A` 1.0) 2.0 "fsafsafd"))

(fn `UserConstructionScript`)