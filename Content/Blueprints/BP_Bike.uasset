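; Player bike for a timed distance challenge, driven along a spline track by a real bike's speed sensor.
; Sustained pedalling starts the race; Tick then converts sensor speed into spline distance, with sine sway and speed-scaled camera FOV and loop audio.
; At time-out it ranks distance and top speed, saves scores, updates the leaderboard and resets after a delay.
; It also handles the HUD, pause menu and debug GI/anti-aliasing toggles.
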(event `self.ReceiveBeginPlay`
  (bind _spline (`self.Spline`))
  (bind _camera (`self.Camera`))
  (bind _distance (`self.Distance`))
  (bind _currentspeed (`self.CurrentSpeed`))
  (bind _currentspeed_2 (`self.CurrentSpeed`))
  (bind _bikeloop (`self.BikeLoop`))
  (`|ExecutionSequence`
    (:`then_0`
      (bind _returnvalue (`GameplayStatics.LoadGameFromSlot` "1"))
      (bind _asbp_save_game (cast `/Game/Blueprints/BP_SaveGame` _returnvalue)
        (:`then`
          (set `self.SaveGame` _asbp_save_game)
          (set `self.RecordedTimes` (`/Game/Blueprints/BP_SaveGame.HighScoreTotalDistance` _asbp_save_game))
          (set `self.TopSpeedRecords` (`/Game/Blueprints/BP_SaveGame.HighScoreTopSpeed` _asbp_save_game)))
        (:`CastFailed`
          (bind _returnvalue_2 (`GameplayStatics.CreateSaveGameObject` "/Game/Blueprints/BP_SaveGame.BP_SaveGame_C"))
          (set `self.SaveGame` _returnvalue_2))))
    (:`then_1`
      (bind _splineactor (`self.SplineActor`)
        (:`then`
          (set `self.Spline` (`/Game/Blueprints/BP_TrackSpline.Spline` _splineactor))
          (bind _asplayer_controller (cast `PlayerController` (`self.GetController`)))
          (message `EnhancedInputSubsystemInterface.AddMappingContext` (pcsubsystem `EnhancedInputLocalPlayerSubsystem` _asplayer_controller) "/Game/Input/IM_Controls.IM_Controls" 0 (struct))
          (set `self.TrackDistance` (`SplineComponent.GetSplineLength` (`self.Spline`)))
          (set `self.TimerCurrent` (`self.TimerMax`))
          (bind _returnvalue_3 (`|CreateWidget` "/Game/Blueprints/WBP_HUD.WBP_HUD_C"))
          (bind _output_get (set `self.HUD` _returnvalue_3))
          (`UserWidget.AddToViewport` _output_get 0)
          (bind _returnvalue_4 (`|CreateWidget` "/Game/Blueprints/WBP_PauseMenu.WBP_PauseMenu_C"))
          (bind _output_get_2 (set `self.PauseMenu` _returnvalue_4))
          (set `/Game/Blueprints/WBP_PauseMenu.Bike` self _output_get_2)
          (`self.UpdateLeaderboard`))
        (:`else`
          (`KismetSystemLibrary.PrintString` "No Spline Track Assigned to Player!" true true (struct :`R` 1.0 :`A` 1.0) 100.0))))
    (:`then_2`
      (bind _output_get_3 (set `self.SwayOffset` (`KismetMathLibrary.MakeVector` 0.0 0.0 (* (`KismetMathLibrary.DegSin` (/ (`self.Distance`) 2.0)) (`self.SwayAmount`))) :!label _label))
      (`self.K2_SetActorLocationAndRotation` (+ (`SplineComponent.GetLocationAtDistanceAlongSpline` _spline _distance "World") _output_get_3) (`SplineComponent.GetRotationAtDistanceAlongSpline` _spline (+ _distance 500.0) "World"))
      (`CameraComponent.SetFieldOfView` _camera (`KismetMathLibrary.Lerp` (`CameraComponent.FieldOfView` _camera) (`KismetMathLibrary.MapRangeClamped` (`self.CurrentSpeed`) 0.0 1.0 90.0 110.0) (* (`GameplayStatics.GetWorldDeltaSeconds`) 5.0)))
      (set `AudioComponent.PitchMultiplier` (`KismetMathLibrary.Lerp` 1.0 2.0 _currentspeed) _bikeloop)
      (`AudioComponent.SetVolumeMultiplier` _bikeloop (`KismetMathLibrary.Lerp` 0.0 2.0 _currentspeed))
      (if (> _currentspeed_2 (`self.TopSpeedThisRace`))
        (set `self.TopSpeedThisRace` _currentspeed_2)))))

(event `self.ReceiveTick`
  (params (DeltaSeconds :type "Float (single-precision)"))
  (bind _returnvalue (`GameplayStatics.GetWorldDeltaSeconds`))
  (bind _timercurrent (`self.TimerCurrent`))
  (set `self.CurrentSpeed` (/ (`BikeSensorComponent.GetSpeedKph` (`self.BikeSensor`)) 100.0))
  (if (`self.RaceFinished`)
    _
    (elif (`self.Racing`)
      (if (<= _timercurrent 0.0)
        (`self.EndRace`)
        (else
          (set `self.TimerCurrent` (- _timercurrent _returnvalue))
          (set `self.Distance` (+ (`self.Distance`) (* _returnvalue (`self.MaxSpeed`) (`self.CurrentSpeed`))))
          (goto _label)))
      (elif (> (`self.CurrentSpeed`) 0.05)
        (set `self.RaceStartTimerCurrent` (+ (`self.RaceStartTimerCurrent`) _returnvalue))
        (if (>= (`self.RaceStartTimerCurrent`) (`self.RaceStartTimerMax`))
          (set `self.Racing` true))
        (else
          (set `self.RaceStartTimerCurrent` 0.0))))))

(event `self.BikeSensor.OnBikeDataUpdated`
  (params (Data :type "BikeCSCData Structure (by ref)")))

(event `Key|N`
  (params (Key :type "Key Structure"))
  (:`Pressed`
    (`/Engine/EditorBlueprintResources/StandardMacros.FlipFlop`
      (:`A`
        (`KismetSystemLibrary.ExecuteConsoleCommand` "r.DynamicGlobalIlluminationMethod 0" null))
      (:`B`
        (`KismetSystemLibrary.ExecuteConsoleCommand` "r.DynamicGlobalIlluminationMethod 1" null)))))

(event `Key|M`
  (params (Key :type "Key Structure"))
  (:`Pressed`
    (`/Engine/EditorBlueprintResources/StandardMacros.FlipFlop`
      (:`A`
        (`KismetSystemLibrary.ExecuteConsoleCommand` "r.antialiasingmethod 2" null))
      (:`B`
        (`KismetSystemLibrary.ExecuteConsoleCommand` "r.antialiasingmethod 4" null)))))

(event `EndRace`
  (bind _recordedtimes (`self.RecordedTimes`))
  (bind _distance (`self.Distance`))
  (bind _topspeedrecords (`self.TopSpeedRecords`))
  (bind _topspeedthisrace (`self.TopSpeedThisRace`))
  (set `self.RaceFinished` true)
  (set `self.Racing` false)
  (set `self.TimerCurrent` 0.0)
  (`KismetArrayLibrary.Array_AddUnique` _topspeedrecords _topspeedthisrace)
  (`KismetArrayLibrary.SortFloatArray` _topspeedrecords false "Descending")
  (`KismetArrayLibrary.Array_AddUnique` _recordedtimes _distance)
  (`KismetArrayLibrary.SortFloatArray` _recordedtimes false "Descending")
  (if (or (== _distance (`|GetArrayItem` _recordedtimes)) (== (`|GetArrayItem` _topspeedrecords) _topspeedthisrace))
    (set `self.EndText` "WORLD RECORD!")
    (elif (>= (/ _distance 100.0) (`self.TokenGoal`))
      (set `self.EndText` "WINNER WINNER, \nOUTBACK DINNER!")
      (else
        (set `self.EndText` "BETTER LUCK NEXT TIME"))))
  (`self.UpdateLeaderboard`)
  (`self.SaveHighScores`)
  (`AudioComponent.SetVolumeMultiplier` (`self.BikeLoop`) 0.0)
  (`KismetSystemLibrary.Delay` 10.0)
  (`self.RestartRace`))

(event `ClearScores`
  (bind _savegame (`self.SaveGame`))
  (`KismetArrayLibrary.Array_Clear` (`self.RecordedTimes`))
  (`KismetArrayLibrary.Array_Clear` (`self.TopSpeedRecords`))
  (`self.UpdateLeaderboard`)
  (set `/Game/Blueprints/BP_SaveGame.HighScoreTotalDistance` (`self.RecordedTimes`) _savegame :!label _label_2)
  (set `/Game/Blueprints/BP_SaveGame.HighScoreTopSpeed` (`self.TopSpeedRecords`) _savegame)
  (`GameplayStatics.SaveGameToSlot` _savegame "1"))

(event `SaveHighScores`
  (goto _label_2))

(event `RestartRace`
  (set `self.RaceFinished` false)
  (set `self.Distance` 0.0)
  (set `self.TimerCurrent` (`self.TimerMax`))
  (`self.SetCameraToDistance` 0.0)
  (set `self.TopSpeedThisRace` 0.0))

(event `Unpause`
  (bind _returnvalue (`GameplayStatics.GetPlayerController` 0))
  (`GameplayStatics.SetGamePaused` false :!label _label_3)
  (`UserWidget.AddToViewport` (`self.HUD`) 0)
  (`Widget.RemoveFromParent` (`self.PauseMenu`))
  (`WidgetBlueprintLibrary.SetInputMode_GameOnly` _returnvalue)
  (set `PlayerController.bShowMouseCursor` false _returnvalue))

(event `EnhancedInput|/Game/Input/IA_Pause`
  (params (ActionValue :type Boolean) (ElapsedSeconds :type "Float (double-precision)") (TriggeredSeconds :type "Float (double-precision)") (InputAction :type "InputAction Object Reference" :default "/Game/Input/IA_Pause.IA_Pause"))
  (bind _returnvalue (`GameplayStatics.GetPlayerController` 0))
  (bind _pausemenu (`self.PauseMenu`))
  (:`Started`
    (if (`GameplayStatics.IsGamePaused`)
      (goto _label_3)
      (else
        (`GameplayStatics.SetGamePaused` true)
        (`Widget.RemoveFromParent` (`self.HUD`))
        (`UserWidget.AddToViewport` _pausemenu 0)
        (`WidgetBlueprintLibrary.SetInputMode_GameAndUIEx` _returnvalue _pausemenu)
        (set `PlayerController.bShowMouseCursor` true _returnvalue)))))

(event `self.BikeSensor.OnBikeConnected`
  (`KismetSystemLibrary.PrintString` "Bike Connected"))

(fn `SetCameraToDistance`
  (params (Distance :type "Float (double-precision)"))
  (bind _spline (`self.Spline`))
  (bind _distance (`self.Distance`))
  (`self.K2_SetActorLocationAndRotation` (`SplineComponent.GetLocationAtDistanceAlongSpline` _spline _distance "World") (`SplineComponent.GetRotationAtDistanceAlongSpline` _spline _distance "World")))

(fn `UserConstructionScript`)